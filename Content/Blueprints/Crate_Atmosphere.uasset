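; Interactable atmosphere crate that, once activated by the player's rover, emits cloud particles and advances the mission.
; It binds to the rover pawn's OnInteract event and responds when the rover is within Proximity.
; Each successful interaction sets Activated and increments Mission on the TaskManager, with no repeat guard.
; While active, Tick repositions SteamEmitter and attaches a new, non-auto-destroyed CloudSpawner emitter every frame.
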(event Custom|OnInteract_Event
  (bind _newparam (CallFunction|InRange))
  (if _newparam
    (Variables|Default|SetActivated true)
    (bind _outactors (Actor|GetAllActorsOfClass "/Game/Blueprints/TaskManager.TaskManager_C"))
    (bind _astaskmanager_c (Utilities|Casting|CastToTaskManager (Utilities|Array|Get(acopy) _outactors)))
    (Variables|/Game/Blueprints/TaskManager.TaskManager_C|SetMission _astaskmanager_c (+ (Variables|/Game/Blueprints/TaskManager.TaskManager_C|GetMission _astaskmanager_c) 1))))

(event EventBeginPlay
  (bind _asrovergamepawn_bp_c (Utilities|Casting|CastToRoverGamePawn_BP (Game|Player|GetPlayerPawn 0)))
  (EventDispatchers|BindEventtoOnInteract _asrovergamepawn_bp_c (delegate Custom|OnInteract_Event)))

(event EventTick
  (params (DeltaSeconds :type Float%20%28single-precision%29))
  (bind _steamemitter (Variables|Default|GetSteamEmitter))
  (if (Variables|Default|GetActivated)
    (Transformation|SetWorldLocation _steamemitter (Transformation|GetActorLocation) false)
    (Transformation|SetRelativeLocation _steamemitter "0, 0,-600.000000" false)
    (Effects|SpawnEmitterAttached "/Game/Particles/CloudSpawner.CloudSpawner" _steamemitter "None" "0, 0,-100.000000" "0, 0, 0" "EAttachLocation::KeepRelativeOffset" false)))

(fn ConstructionScript)

(fn InRange
  (bind _asrovergamepawn_bp_c (Utilities|Casting|CastToRoverGamePawn_BP (Game|Player|GetPlayerPawn 0)))
  (bind _returnvalue (Transformation|GetDistanceTo _asrovergamepawn_bp_c))
  (if (< _returnvalue (Variables|Default|GetProximity))
    (LocalVariables|SetretVal true)
    (else
      (LocalVariables|SetretVal false)))
  (return (LocalVariables|GetretVal)))