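; Crate actor that shakes the rover's camera when nearby until the player interacts with it to advance the mission.
; Each tick, while unactivated and within Proximity, it alternates a random vertical camera offset scaled by ShakeMagnitude with a stored LastShake offset.
; It binds to the rover pawn's OnInteract event; an in-range interaction sets Activated, stopping the shake, and sets the TaskManager's Mission to 2.
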(event Custom|OnInteract_Event
  (bind _newparam (CallFunction|InRange))
  (if _newparam
    (Variables|Default|SetActivated true)
    (bind _outactors (Actor|GetAllActorsOfClass "/Game/Blueprints/TaskManager.TaskManager_C"))
    (bind _astaskmanager_c (Utilities|Casting|CastToTaskManager (Utilities|Array|Get(acopy) _outactors)))
    (Variables|/Game/Blueprints/TaskManager.TaskManager_C|SetMission _astaskmanager_c 2)))

(event EventBeginPlay
  (bind _asrovergamepawn_bp_c (Utilities|Casting|CastToRoverGamePawn_BP (Game|Player|GetPlayerPawn 0)))
  (EventDispatchers|BindEventtoOnInteract _asrovergamepawn_bp_c (delegate Custom|OnInteract_Event)))

(event EventTick
  (params (DeltaSeconds :type Float%20%28single-precision%29))
  (CallFunction|VibrateCamera))

(fn ConstructionScript)

(fn VibrateCamera
  (bind _returnvalue (Math|Random|RandomFloatinRange -1.0 1.0))
  (bind _shake_magnitude (Variables|Default|GetShake%20Magnitude))
  (bind _returnvalue_2 (|rnd*magnitude _returnvalue _shake_magnitude))
  (bind _returnvalue_3 (Math|Vector|MakeVector 0.0 0.0 _returnvalue_2))
  (bind _asrovergamepawn_bp_c (Utilities|Casting|CastToRoverGamePawn_BP (Game|Player|GetPlayerPawn 0)))
  (bind _newparam (CallFunction|InRange))
  (if (and (not (Variables|Default|GetActivated)) _newparam)
    (if (Variables|Default|GetRebound)
      (Variables|Default|SetRebound (not (Variables|Default|GetRebound)))
      (Transformation|AddLocalOffset (Variables|/Script/RoverGame.RoverGamePawn|GetCamera _asrovergamepawn_bp_c) (Variables|Default|GetLastShake) false)
      (else
        (Transformation|AddLocalOffset (Variables|/Script/RoverGame.RoverGamePawn|GetCamera _asrovergamepawn_bp_c) _returnvalue_3 false)
        (Variables|Default|SetLastShake _returnvalue_3)
        (Variables|Default|SetRebound (not (Variables|Default|GetRebound)))))))

(fn InRange
  (bind _returnvalue (Game|Player|GetPlayerPawn 0))
  (Utilities|Casting|CastToRoverGamePawn_BP _returnvalue)
  (bind _returnvalue_2 (Transformation|GetDistanceTo _returnvalue))
  (if (< _returnvalue_2 (Variables|Default|GetProximity))
    (LocalVariables|SetretVal true)
    (else
      (LocalVariables|SetretVal false)))
  (return (LocalVariables|GetretVal)))