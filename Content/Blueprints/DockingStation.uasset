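; Docking station that recharges the player rover's energy while docked.
; A trigger box sets the docked flag on begin and end overlap, without checking which actor overlaps.
; While docked, Tick feeds the rover pawn's energy and the charging rate into EnergyRecharge each frame whenever energy is below 100, with no delta-time scaling in the call.
; The Interact input checks the docked flag but performs no action.
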(event OnComponentEndOverlap(TriggerBox)
  (params (OtherActor :type Actor%20Object%20Reference) (OtherComp :type Primitive%20Component%20Object%20Reference) (OtherBodyIndex :type Integer))
  (Variables|Default|SetDocked false))

(event OnComponentBeginOverlap(TriggerBox)
  (params (OtherActor :type Actor%20Object%20Reference) (OtherComp :type Primitive%20Component%20Object%20Reference) (OtherBodyIndex :type Integer) (bFromSweep :type Boolean) (SweepResult :type Hit%20Result%20Structure%20%28by%20ref%29))
  (Variables|Default|SetDocked true))

(event EventTick
  (params (DeltaSeconds :type Float%20%28single-precision%29))
  (bind _asrovergamepawn_bp_c (Utilities|Casting|CastToRoverGamePawn_BP (Game|Player|GetPlayerPawn 0)))
  (if (and (Variables|Default|GetDocked) (< (Variables|/Game/Blueprints/RoverGamePawn_BP.RoverGamePawn_BP_C|GetEnergy _asrovergamepawn_bp_c) 1e+02))
    (Variables|/Game/Blueprints/RoverGamePawn_BP.RoverGamePawn_BP_C|SetEnergy _asrovergamepawn_bp_c (|Energy+Recharge (Variables|/Game/Blueprints/RoverGamePawn_BP.RoverGamePawn_BP_C|GetEnergy _asrovergamepawn_bp_c) (Variables|Default|GetChargingRate)))))

(event Input|ActionEvents|InputActionInteract
  (:Pressed
    (if (Variables|Default|GetDocked)
      _)))

(fn ConstructionScript)