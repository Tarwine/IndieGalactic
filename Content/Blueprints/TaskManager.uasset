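; TaskManager is an actor Blueprint that spawns world objects for the active mission.
; Every tick it switches on the Mission number and calls the matching mission function, each guarded by a started flag so it runs once.
; Missions one and two each spawn a crate, tectonics then atmosphere, at fixed coordinates.
; Mission three spawns a row of seed ammo pickups along X.
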(event EventTick
  (params (DeltaSeconds :type Float%20%28single-precision%29))
  (switch int (Variables|Default|GetMission)
    (:1
      (CallFunction|Mission1))
    (:2
      (CallFunction|Mission2))
    (:3
      (CallFunction|Mission3))))

(fn ConstructionScript)

(fn Mission1
  (if (not (Variables|Default|GetTask1Started))
    (Variables|Default|SetTask1Started true)
    (Game|SpawnActorfromClass "/Game/Blueprints/Crate_Techtonics.Crate_Techtonics_C" (Math|Conversions|ToTransform(Vector) (Math|Vector|MakeVector 2.104e+04 0.0 1e+03)) false)))

(fn Mission2
  (if (not (Variables|Default|GetTask2Started))
    (Variables|Default|SetTask2Started true)
    (Game|SpawnActorfromClass "/Game/Blueprints/Crate_Atmosphere.Crate_Atmosphere_C" (Math|Conversions|ToTransform(Vector) (Math|Vector|MakeVector 5.91e+03 -2.667e+04 1e+03)) false)))

(fn Mission3
  (if (not (Variables|Default|GetTask3Started))
    (Variables|Default|SetTask3Started true)
    (for _index (range 0 10)
      (Game|SpawnActorfromClass "/Game/Blueprints/SeedAmmo.SeedAMmo_C" (Math|Conversions|ToTransform(Vector) (Math|Vector|MakeVector (Math|Conversions|ToFloat(Integer) (+ (* _index 100) 8450)) -1.628e+04 1e+02)) true))))